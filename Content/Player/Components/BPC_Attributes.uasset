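; Player attributes component that tracks health, mana and death state, starting both pools at their maximums on BeginPlay.
; ReceiveDamage, RestoreHealth and RestoreMana clamp their values, while TrySpendMana deducts only affordable costs and returns success.
; Changes broadcast OnHealthChanged or OnManaChanged, and reaching zero health sets IsDead and fires OnDeath.
; Once dead, damage, restoration and mana spending are all blocked.
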(event EventBeginPlay
  ;[0.15 0.15 0.15 0.5] Инициализация
  (Variables|Default|SetCurrentHealth (Variables|Default|GetMaxHealth))
  (Variables|Default|SetCurrentMana (Variables|Default|GetMaxMana))
  (Variables|Default|SetIsDead false))

(event EventTick
  (params (DeltaSeconds :type Float%20%28single-precision%29)))

(fn ReceiveDamage
  (params (DamageAmount :type Float%20%28double-precision%29))
  (if (and (> DamageAmount 0.0) (not (Variables|Default|GetIsDead)))
    (bind _output_get (Variables|Default|SetCurrentHealth (Math|Float|Clamp(Float) (- (Variables|Default|GetCurrentHealth) DamageAmount) 0.0 (Variables|Default|GetMaxHealth))))
    (Default|CallOnHealthChanged _output_get (Variables|Default|GetMaxHealth))
    (if (<= (Variables|Default|GetCurrentHealth) 0.0)
      (Variables|Default|SetIsDead true)
      (Default|CallOnDeath))))

(fn TrySpendMana
  (params (ManaCost :type Float%20%28double-precision%29))
  (if (Math|Boolean|ANDBoolean (>= ManaCost 0.0) (>= (Variables|Default|GetCurrentMana) ManaCost) (not (Variables|Default|GetIsDead)))
    (bind _output_get (Variables|Default|SetCurrentMana (- (Variables|Default|GetCurrentMana) ManaCost)))
    (Default|CallOnManaChanged _output_get (Variables|Default|GetMaxMana))
    (return true)
    (else
      (Development|PrintString "Not enough mana")
      (return false))))

(fn RestoreHealth
  (params (Amount :type Float%20%28double-precision%29))
  (if (and (> Amount 0.0) (not (Variables|Default|GetIsDead)))
    (bind _output_get (Variables|Default|SetCurrentHealth (Math|Float|Clamp(Float) (+ (Variables|Default|GetCurrentHealth) Amount) 0.0 (Variables|Default|GetMaxHealth))))
    (Default|CallOnHealthChanged _output_get (Variables|Default|GetMaxHealth))))

(fn RestoreMana
  (params (Amount :type Float%20%28double-precision%29))
  (if (and (> Amount 0.0) (not (Variables|Default|GetIsDead)))
    (bind _output_get (Variables|Default|SetCurrentMana (Math|Float|Clamp(Float) (+ (Variables|Default|GetCurrentMana) Amount) 0.0 (Variables|Default|GetMaxMana))))
    (Default|CallOnManaChanged _output_get (Variables|Default|GetMaxMana))))