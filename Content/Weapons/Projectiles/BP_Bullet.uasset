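; BP_Bullet is a weapon projectile that damages the actor it hits.
; On BeginPlay, its collision component ignores the owner during movement, and a Character owner's capsule ignores the bullet in return, avoiding collisions with the shooter.
; On a component hit, it applies ProjectileDamage to any non-owner actor, crediting the instigator's controller, and destroys itself whatever it hit.
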(event OnComponentHit(BulletCollision)
  (params (HitComponent :type Primitive%20Component%20Object%20Reference) (OtherActor :type Actor%20Object%20Reference) (OtherComp :type Primitive%20Component%20Object%20Reference) (NormalImpulse :type Vector :default "0, 0, 0") (Hit :type Hit%20Result%20Structure%20%28by%20ref%29))
  (if (!= OtherActor (Components|GetOwner))
    (Game|Damage|ApplyDamage OtherActor (Variables|Default|GetProjectileDamage) (Game|GetInstigatorController) self)
    (Actor|DestroyActor)
    (else
      (Actor|DestroyActor))))

(event EventBeginPlay
  (Collision|IgnoreActorwhenMoving (Variables|Default|GetBulletCollision) (Components|GetOwner) true)
  (bind _ascharacter (Utilities|Casting|CastToCharacter (Components|GetOwner)))
  (Collision|IgnoreActorwhenMoving (Variables|/Script/Engine.Character|GetCapsuleComponent _ascharacter) self true))

(event Collision|EventActorBeginOverlap
  (params (OtherActor :type Actor%20Object%20Reference)))

(event EventTick
  (params (DeltaSeconds :type Float%20%28single-precision%29)))

(fn ConstructionScript)