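; BP_Sword is a melee weapon Blueprint that deals area damage on its primary attack.
; PerformPrimaryAttack runs a multi-sphere object trace forward from AttackOrigin over AttackRange, detecting Pawns and ignoring the owner.
; Each hit receives Damage through ApplyDamage, credited to the instigator's controller with the sword as causer.
; The trace draws timed debug shapes, and hits are not de-duplicated by actor.
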(event EventPerformPrimaryAttack
  (bind _attackorigin (Variables|Default|GetAttackOrigin))
  (bind _returnvalue (Transformation|GetWorldLocation _attackorigin))
  (bind _outhits (Collision|MultiSphereTraceForObjects _returnvalue (+ _returnvalue (* (Math|Vector|GetForwardVector _attackorigin) (Variables|Default|GetAttackRange))) (Variables|Default|GetAttackRadius) (Utilities|Array|MakeArray "ObjectTypeQuery3") false (Utilities|Array|MakeArray (Components|GetOwner)) "ForDuration"))
  (for _array_element _outhits
    (Game|Damage|ApplyDamage (.HitActor (Collision|BreakHitResult _array_element)) (Variables|Default|GetDamage) (Game|GetInstigatorController) self)))

(fn ConstructionScript
  (|CallParentFunction))